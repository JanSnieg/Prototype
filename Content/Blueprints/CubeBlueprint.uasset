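; Selectable cube actor that the player picks as a guess, deciding win or lose when its own child sphere leaves its box.
; Click or touch selects it if no cube is active, or deselects it before the Flex emitter simulation starts, updating the HUD.
; A dynamic material shows selection and hover.
; The sphere's exit sets the player controller's end text by selection state and ends the game.
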(event `self.ReceiveBeginPlay`
  ;[1 1 1] Setting material on start
  (bind _returnvalue (`PrimitiveComponent.CreateDynamicMaterialInstance` (`self.Container`) 0 "/Game/Materials/CubeBasic-_Inst.CubeBasic-_Inst"))
  (set `self.Material` _returnvalue)
  (`self.SetOwner` (`ChildActorComponent.ChildActor` (`self.shpere`)) self))

(event `self.Container.OnInputTouchBegin`
  (params (FingerIndex :type "ETouchIndex Enum" :default "Touch1") (TouchedComponent :type "PrimitiveComponent Object Reference"))
  ;[1 1 1] Checking if is possible to select
  (bind _isactive (`self.isAnyActive` :!label _label))
  (if _isactive
    (bind _isstarted (`self.isSimulationStarted`))
    (if (not _isstarted)
      ;[1 1 1] Block/Unblock clicked
      (if (`self.isActive`)
        (set `self.isActive` false)
        (`MaterialInstanceDynamic.SetVectorParameterValue` (`self.Material`) (`self.Glass`) (`self.GlassBasic`))
        (bind _foundwidgets (`WidgetBlueprintLibrary.GetAllWidgetsWithInterface` "/Game/Blueprints/PlayerInterface.PlayerInterface_C"))
        (bind _ashud (cast `/Game/UI/HUD` (`|GetArrayItem` _foundwidgets)))
        (set `/Game/UI/HUD.isSelected` false _ashud)))
    (else
      (set `self.isActive` true)
      (`MaterialInstanceDynamic.SetVectorParameterValue` (`self.Material`) (`self.Glass`) (`self.GlassSelected`))
      (bind _foundwidgets_2 (`WidgetBlueprintLibrary.GetAllWidgetsWithInterface` "/Game/Blueprints/PlayerInterface.PlayerInterface_C"))
      (bind _ashud_2 (cast `/Game/UI/HUD` (`|GetArrayItem` _foundwidgets_2)))
      (set `/Game/UI/HUD.isSelected` true _ashud_2))))

(event `self.container.OnClicked`
  (params (TouchedComponent :type "PrimitiveComponent Object Reference") (ButtonPressed :type "Key Structure"))
  ;[1 1 1] Checking if is possible to select
  (goto _label))

(event `self.container.OnBeginCursorOver`
  (params (TouchedComponent :type "PrimitiveComponent Object Reference"))
  ;[1 1 1] Highlighting when mouseover
  (if (not (`self.isHighlited`))
    (`MaterialInstanceDynamic.SetVectorParameterValue` (`self.Material`) (`self.Border`) (`self.BorderSelected`))
    (set `self.isHighlited` true)))

(event `self.container.OnEndCursorOver`
  (params (TouchedComponent :type "PrimitiveComponent Object Reference"))
  ;[1 1 1] Highlighting when mouseover
  (if (`self.isHighlited`)
    (`MaterialInstanceDynamic.SetVectorParameterValue` (`self.Material`) (`self.Border`) (`self.BorderBasic`))
    (set `self.isHighlited` false)))

(event `self.Box.OnComponentEndOverlap`
  (params (OverlappedComponent :type "PrimitiveComponent Object Reference") (OtherActor :type "Actor Object Reference") (OtherComp :type "PrimitiveComponent Object Reference") (OtherBodyIndex :type Integer))
  (bind _returnvalue (`GameplayStatics.GetPlayerController` 0))
  ;[1 1 1] Win Conditions
  (if (== (`ActorComponent.GetOwner` OverlappedComponent) (`self.GetOwner` OtherActor))
    (if (`self.isActive`)
      (bind _asplayercontroller (cast `/Game/Blueprints/playercontroller` _returnvalue))
      (set `/Game/Blueprints/playercontroller.EndText` "YOU WON!" _asplayercontroller)
      (else
        (bind _asplayercontroller_2 (cast `/Game/Blueprints/playercontroller` _returnvalue))
        (set `/Game/Blueprints/playercontroller.EndText` "YOU LOSE!" _asplayercontroller_2)))
    (`/Game/Blueprints/playercontroller.EndGame` _asplayercontroller)
    (`/Game/Blueprints/playercontroller.EndGame` _asplayercontroller_2)))

(fn `isAnyActive`
  (returns (isActive :type Boolean))
  (bind _outactors (`GameplayStatics.GetAllActorsOfClass` "CubeBlueprint_C"))
  (for _array_element _outactors
    (if (`/Game/Blueprints/CubeBlueprint.isActive` _array_element)
      (return true)))
  (return false))

(fn `isSimulationStarted`
  (returns (isStarted :type Boolean))
  (bind _outactors (`GameplayStatics.GetAllActorsWithInterface` "/Game/Blueprints/PlayerInterface.PlayerInterface_C"))
  (bind _asflex_emitter (cast `/Game/Blueprints/flexEmitter` (`|GetArrayItem` _outactors)))
  (return (`ActorComponent.IsActive` (`Emitter.ParticleSystemComponent` _asflex_emitter))))

(fn `UserConstructionScript`)