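; CameraPawn is a pawn that provides a mouse-wheel zoom camera and sets up the player's HUD.
; On BeginPlay it adds the HUD widget, switches to game-only input with a visible cursor, and narrowly limits camera manager pitch and roll.
; Wheel presses step the spring arm's length within a clamped range and derive its vertical target offset from that new length, so height changes with zoom.
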(event `self.ReceiveBeginPlay`
  (bind _returnvalue (`GameplayStatics.GetPlayerCameraManager` 0))
  (bind _returnvalue_2 (`GameplayStatics.GetPlayerController` 0))
  (bind _returnvalue_3 (`|CreateWidget` "/Game/UI/HUD.HUD_C"))
  (bind _output_get (set `self.HUDReference` _returnvalue_3))
  (`UserWidget.AddToViewport` _output_get 0)
  (`WidgetBlueprintLibrary.SetInputMode_GameOnly` _returnvalue_2)
  (set `PlayerController.bShowMouseCursor` true _returnvalue_2)
  ;[1 1 1] Limiting camera
  (set `PlayerCameraManager.ViewPitchMax` 10.0 _returnvalue)
  (set `PlayerCameraManager.ViewPitchMin` -10.0 _returnvalue)
  (set `PlayerCameraManager.ViewRollMax` 10.0 _returnvalue)
  (set `PlayerCameraManager.ViewRollMin` -10.0 _returnvalue))

(event `Key|MouseScrollDown`
  (params (Key :type "Key Structure"))
  (bind _springarm (`self.SpringArm`))
  (bind _returnvalue (`KismetMathLibrary.FClamp` (+ (`SpringArmComponent.TargetArmLength` _springarm) 25.0) 300.0 600.0))
  (:`Pressed`
    (set `SpringArmComponent.TargetArmLength` _returnvalue _springarm)
    (set `SpringArmComponent.TargetOffset` (`KismetMathLibrary.MakeVector` 0.0 0.0 _returnvalue) _springarm)))

(event `Key|MouseScrollUp`
  (params (Key :type "Key Structure"))
  (bind _springarm (`self.SpringArm`))
  (bind _returnvalue (`KismetMathLibrary.FClamp` (- (`SpringArmComponent.TargetArmLength` _springarm) 25.0) 300.0 600.0))
  (:`Pressed`
    (set `SpringArmComponent.TargetArmLength` _returnvalue _springarm)
    (set `SpringArmComponent.TargetOffset` (`KismetMathLibrary.MakeVector` 0.0 0.0 _returnvalue) _springarm)))

(fn `UserConstructionScript`)