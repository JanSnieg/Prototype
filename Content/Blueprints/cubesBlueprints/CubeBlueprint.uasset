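; Selectable glass cube holding a child-actor duck, used as the player's pick in a game decided by which duck leaves its cube.
; Clicking toggles or moves the single active selection, updating glass color and HUD; an existing selection locks while the FlexEmitter simulation runs.
; Hovering highlights the border through a dynamic material.
; When its own duck exits the Box, it ends the game through Playercontroller, winning if this cube is active, losing otherwise.
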(event `self.ReceiveBeginPlay`
  ;[1 1 1] Setting material on start
  (bind _returnvalue (`PrimitiveComponent.CreateDynamicMaterialInstance` (`self.Container`) 0 "/Game/Materials/CubeBasic-_Inst.CubeBasic-_Inst"))
  (set `self.Material` _returnvalue)
  ;[1 1 1] Setting Owner for duck
  (`self.SetOwner` (`ChildActorComponent.ChildActor` (`self.shpere`)) self))

(event `self.container.OnClicked`
  (params (TouchedComponent :type "PrimitiveComponent Object Reference") (ButtonPressed :type "Key Structure"))
  ;[1 1 1] Checking if is possible to select
  (bind _isactive (`self.isAnyActive`))
  (if _isactive
    (bind _isstarted (`self.isSimulationStarted`))
    (if (not _isstarted)
      ;[1 1 1] Block/Unblock clicked
      (if (`self.isActive`)
        (`GameplayStatics.PlaySound2D` "/Game/Music/FX/switch13.switch13")
        (`self.Desactivate`)
        (else
          (`self.Reclick`)))
      (bind _foundwidgets (`WidgetBlueprintLibrary.GetAllWidgetsOfClass` "/Game/UI/HUD.HUD_C" :!label _label))
      (set `/Game/UI/HUD.isSelected` (`self.isActive`) (`|GetArrayItem` _foundwidgets)))
    (else
      (`GameplayStatics.PlaySound2D` "/Game/Music/FX/switch12.switch12")
      (`self.Activate`)
      (goto _label))))

(event `self.container.OnBeginCursorOver`
  (params (TouchedComponent :type "PrimitiveComponent Object Reference"))
  ;[1 1 1] Highlighting when mouseover
  (`GameplayStatics.PlaySound2D` "/Game/Music/FX/rollover4.rollover4")
  (if (not (`self.isHighlited`))
    (`MaterialInstanceDynamic.SetVectorParameterValue` (`self.Material`) (`self.Border`) (`self.BorderSelected`))
    (set `self.isHighlited` true)))

(event `self.container.OnEndCursorOver`
  (params (TouchedComponent :type "PrimitiveComponent Object Reference"))
  ;[1 1 1] Highlighting when mouseover
  (if (`self.isHighlited`)
    (`MaterialInstanceDynamic.SetVectorParameterValue` (`self.Material`) (`self.Border`) (`self.BorderBasic`))
    (set `self.isHighlited` false)))

(event `self.Box.OnComponentEndOverlap`
  (params (OverlappedComponent :type "PrimitiveComponent Object Reference") (OtherActor :type "Actor Object Reference") (OtherComp :type "PrimitiveComponent Object Reference") (OtherBodyIndex :type Integer))
  ;[1 1 1] Win Conditions
  (if (== (`ActorComponent.GetOwner` OverlappedComponent) (`self.GetOwner` OtherActor))
    (bind _outactors (`GameplayStatics.GetAllActorsOfClass` "/Game/Blueprints/playercontroller.playercontroller_C"))
    (if (`self.isActive`)
      (bind _output (`|GetArrayItem` _outactors))
      (set `/Game/Blueprints/playercontroller.EndText` "YOU WON!" _output)
      (set `/Game/Blueprints/playercontroller.sfx` "/Game/Music/FX/you_win.you_win" _output)
      (else
        (set `/Game/Blueprints/playercontroller.EndText` "YOU LOSE!" _output)
        (set `/Game/Blueprints/playercontroller.sfx` "/Game/Music/FX/you_lose.you_lose" _output)))
    (`/Game/Blueprints/playercontroller.EndGame` _output)
    (`/Game/Blueprints/playercontroller.EndGame` _output)))

(fn `Activate`
  (set `self.isActive` true)
  (`MeshComponent.SetVectorParameterValueOnMaterials` (`self.Container`) (`self.Glass`) (`KismetMathLibrary.Conv_LinearColorToVector` (`self.GlassSelected`)))
  (`GameplayStatics.PlaySound2D` "/Game/Music/FX/ready.ready")
  (`SceneComponent.SetVisibility` (`self.shpere`) true false))

(fn `Desactivate`
  (`MeshComponent.SetVectorParameterValueOnMaterials` (`self.Container`) (`self.Glass`) (`KismetMathLibrary.Conv_LinearColorToVector` (`self.GlassBasic`)))
  (set `self.isActive` false)
  (`SceneComponent.SetVisibility` (`self.shpere`) false false))

(fn `isAnyActive`
  (returns (isActive :type Boolean))
  (bind _outactors (`GameplayStatics.GetAllActorsOfClass` "CubeBlueprint_C"))
  (for _array_element _outactors
    (if (`/Game/Blueprints/cubesBlueprints/CubeBlueprint.isActive` _array_element)
      (return true)))
  (return false))

(fn `isSimulationStarted`
  (returns (isStarted :type Boolean))
  (bind _outactors (`GameplayStatics.GetAllActorsOfClass` "/Game/Blueprints/flexEmitter.flexEmitter_C"))
  (return (`ActorComponent.IsActive` (`Emitter.ParticleSystemComponent` (`|GetArrayItem` _outactors)))))

(fn `Reclick`
  (bind _outactors (`GameplayStatics.GetAllActorsOfClass` "CubeBlueprint_C"))
  (for _array_element _outactors
    (`self.Desactivate` _array_element))
  (`self.Activate`))

(fn `UserConstructionScript`)