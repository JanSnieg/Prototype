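; movingCamera is a Blueprint that handles pausing and resuming the game; despite its name, it holds no camera movement logic.
; The PauseMenu input calls PauseGame, which pauses, creates the menu widget after a validity check, caches it, displays it and switches to UI-only input.
; UnPauseGame, not called within this graph, resumes play, removes all widgets and restores game-only input.
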(event `InputAction|PauseMenu`
  (params (Key :type "Key Structure"))
  ;[1 1 1] Pause the game
  (:`Pressed`
    (`self.PauseGame`)))

(fn `PauseGame`
  (`GameplayStatics.SetGamePaused` true)
  (`/Engine/EditorBlueprintResources/StandardMacros.IsValid` null
    (:`Is Valid`
      _)
    (:`Is Not Valid`
      (bind _returnvalue (`|CreateWidget` "/Game/UI/PauseMenu.PauseMenu_C" (`GameplayStatics.GetPlayerController` 0)))
      (set `self.PauseMenu` _returnvalue)))
  (`UserWidget.AddToViewport` (`self.PauseMenu`) 0)
  (`WidgetBlueprintLibrary.SetInputMode_UIOnlyEx` (`GameplayStatics.GetPlayerController` 0) (`self.PauseMenu`)))

(fn `UnPauseGame`
  (`GameplayStatics.SetGamePaused` false)
  (`WidgetLayoutLibrary.RemoveAllWidgets`)
  (`WidgetBlueprintLibrary.SetInputMode_GameOnly` (`GameplayStatics.GetPlayerController` 0)))

(fn `UserConstructionScript`)