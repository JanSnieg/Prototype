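; Clickable cube Blueprint that highlights under the cursor and can be selected by clicking.
; Cursor-over events on the Container component swap basic and highlighted materials until the cube becomes active.
; A click locks it active, applies the selected material and sets IsSelected on the HUD widget, found through a PlayerInterface widget search.
; Overlaps on the Cube component only print debug names and a greeting.
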(event `self.container.OnClicked`
  (params (TouchedComponent :type "PrimitiveComponent Object Reference") (ButtonPressed :type "Key Structure"))
  ;[1 1 1] Block clicked
  (if (not (`self.isActive`))
    (set `self.isActive` true)
    (`PrimitiveComponent.SetMaterial` TouchedComponent 0 "/Game/Materials/CubeSelected.CubeSelected")
    (bind _foundwidgets (`WidgetBlueprintLibrary.GetAllWidgetsWithInterface` "/Game/Blueprints/PlayerInterface.PlayerInterface_C"))
    (bind _ashud (cast `/Game/UI/HUD` (`|GetArrayItem` _foundwidgets)))
    (set `/Game/UI/HUD.isSelected` true _ashud)))

(event `self.container.OnBeginCursorOver`
  (params (TouchedComponent :type "PrimitiveComponent Object Reference"))
  ;[1 1 1] Highlighting when mouseover
  (if (`self.isActive`)
    _
    (elif (not (`self.isHighlited`))
      (`PrimitiveComponent.SetMaterial` (`self.container`) 0 "/Game/Materials/CubeHighlited.CubeHighlited")
      (set `self.isHighlited` true))))

(event `self.container.OnEndCursorOver`
  (params (TouchedComponent :type "PrimitiveComponent Object Reference"))
  ;[1 1 1] Highlighting when mouseover
  (if (`self.isActive`)
    _
    (elif (`self.isHighlited`)
      (`PrimitiveComponent.SetMaterial` (`self.container`) 0 "/Game/Materials/CubeBasic.CubeBasic")
      (set `self.isHighlited` false))))

(event `self.Cube.OnComponentBeginOverlap`
  (params (OverlappedComponent :type "PrimitiveComponent Object Reference") (OtherActor :type "Actor Object Reference") (OtherComp :type "PrimitiveComponent Object Reference") (OtherBodyIndex :type Integer) (bFromSweep :type Boolean) (SweepResult :type "HitResult Structure (by ref)"))
  (`KismetSystemLibrary.PrintString` (`KismetSystemLibrary.GetDisplayName` self))
  (`KismetSystemLibrary.PrintString` "Hello")
  (`KismetSystemLibrary.PrintString` (`KismetSystemLibrary.GetDisplayName` OtherActor)))

(fn `UserConstructionScript`)