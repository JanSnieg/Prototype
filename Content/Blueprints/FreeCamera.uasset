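; FreeCamera is a free-flying camera pawn that creates the HUD widget and sets game-only input on BeginPlay.
; Axis inputs add movement along the actor's forward, right and up vectors, and feed controller yaw and pitch.
; Tick consumes the accumulated input vector as a raw, unswept world offset with no delta-time scaling, so speed depends on frame rate.
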(event `self.ReceiveBeginPlay`
  (bind _returnvalue (`|CreateWidget` "/Game/UI/HUD.HUD_C"))
  (bind _output_get (set `self.HUD Reference` _returnvalue))
  (`UserWidget.AddToViewport` _output_get 0)
  (`WidgetBlueprintLibrary.SetInputMode_GameOnly` (`GameplayStatics.GetPlayerController` 0)))

(event `self.ReceiveTick`
  (params (DeltaSeconds :type "Float (single-precision)"))
  (bind _returnvalue (`self.ConsumeMovementInputVector`))
  (`self.K2_AddActorWorldOffset` _returnvalue))

(event `InputAxis|MoveForward`
  (params (AxisValue :type "Float (single-precision)"))
  (`self.AddMovementInput` (`KismetMathLibrary.GetForwardVector` (`self.K2_GetActorRotation`)) AxisValue))

(event `InputAxis|MoveRight`
  (params (AxisValue :type "Float (single-precision)"))
  (`self.AddMovementInput` (`KismetMathLibrary.GetRightVector` (`self.K2_GetActorRotation`)) AxisValue))

(event `InputAxis|RotationX`
  (params (AxisValue :type "Float (single-precision)"))
  (`self.AddControllerYawInput` AxisValue))

(event `InputAxis|MoveUp`
  (params (AxisValue :type "Float (single-precision)"))
  (`self.AddMovementInput` (`KismetMathLibrary.GetUpVector` (`self.K2_GetActorRotation`)) AxisValue))

(event `InputAxis|RotationY`
  (params (AxisValue :type "Float (single-precision)"))
  (`self.AddControllerPitchInput` AxisValue))

(fn `UserConstructionScript`)