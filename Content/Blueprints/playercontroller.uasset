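; Player controller that drives a mouse-panned camera and handles the pause menu.
; On BeginPlay it shows and centers the cursor, then each tick offsets the movingCamera pawn's spring arm from a start location by the scaled viewport mouse position, with vertical inverted.
; The PauseMenu input pauses the game, creates or reuses the menu widget and switches to UI-only input.
; UnPauseGame removes the menu and restores game-only input.
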(event `self.ReceiveBeginPlay`
  (bind (_x _y) (`KismetMathLibrary.BreakVector2D` (`WidgetLayoutLibrary.GetViewportSize`)))
  ;[1 1 1] Camera starting location
  (set `self.bShowMouseCursor` true)
  (set `self.StartLocation` (0.0 -500.0 0.0))
  (`self.SetMouseLocation` (`GameplayStatics.GetPlayerController` 0) (`KismetMathLibrary.FTrunc` (/ _x 2.0)) (`KismetMathLibrary.FTrunc` (/ _y 2.0))))

(event `self.ReceiveTick`
  (params (DeltaSeconds :type "Float (single-precision)"))
  (bind _mousemultiplyer (`self.mouseMultiplyer`))
  ;[1 1 1] MovingCamera
  (bind _returnvalue (`WidgetLayoutLibrary.GetMousePositionOnViewport`))
  (bind _asmoving_camera (cast `/Game/Blueprints/movingCamera` (`GameplayStatics.GetPlayerPawn` 0)))
  (bind (_x _y) (`KismetMathLibrary.BreakVector2D` _returnvalue))
  (`SceneComponent.K2_SetRelativeLocation` (`/Game/Blueprints/movingCamera.SpringArm` _asmoving_camera) (+ (`self.StartLocation`) (`KismetMathLibrary.MakeVector` 0.0 (* _x _mousemultiplyer) (* _y (* _mousemultiplyer -1.0)))) false false))

(event `InputAction|PauseMenu`
  (params (Key :type "Key Structure"))
  ;[1 1 1] Pause the game
  (:`Pressed`
    (`self.PauseGame`)))

(fn `PauseGame`
  (`GameplayStatics.SetGamePaused` true)
  (`/Engine/EditorBlueprintResources/StandardMacros.IsValid` null
    (:`Is Valid`
      _)
    (:`Is Not Valid`
      (bind _returnvalue (`|CreateWidget` "/Game/UI/PauseMenu.PauseMenu_C" (`GameplayStatics.GetPlayerController` 0)))
      (set `self.PauseMenu` _returnvalue)))
  (`UserWidget.AddToViewport` (`self.PauseMenu`) 0)
  (`WidgetBlueprintLibrary.SetInputMode_UIOnlyEx` (`GameplayStatics.GetPlayerController` 0) (`self.PauseMenu`)))

(fn `UnPauseGame`
  (`GameplayStatics.SetGamePaused` false)
  (`Widget.RemoveFromParent` (`self.PauseMenu`))
  (`WidgetBlueprintLibrary.SetInputMode_GameOnly` (`GameplayStatics.GetPlayerController` 0)))

(fn `UserConstructionScript`)